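; Mind control status effect for the turn-based tile toolkit that temporarily makes the affected unit AI-controlled and gives it the controller's allegiances.
; Activation saves the unit's allied factions and AI flag, then copies factions from ControllingUnit, falling back to the active unit.
; Activation and turn start queue a possession emitter, sound and delay through the action manager.
; Turn end restores the saved state and disables the effect.
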(event `self.RunOnTurnStart`
  (`/Game/AdvancedTurnBasedTileToolkit/Core/BP_ActionManager.QueueSpawnEmitter` (`.ActionManager` (`/Game/AdvancedTurnBasedTileToolkit/Core/BPFL_Singletons.GetActionManager2`)) (`KismetMathLibrary.Conv_VectorToTransform` (+ (`self.K2_GetActorLocation` (`/Game/AdvancedTurnBasedTileToolkit/Core/Units/BP_Unit.Puppet` (`self.OwningUnit`))) (0.0 0.0 200.0))) "/Game/AdvancedTurnBasedTileToolkit/Maps/Advanced/Abilities/PS_Posseser_Attach.PS_Posseser_Attach" true true "/Game/AdvancedTurnBasedTileToolkit/Maps/Advanced/Abilities/A_MindControl.A_MindControl" -1.0 :!label _label)
  (`/Game/AdvancedTurnBasedTileToolkit/Core/BP_ActionManager.QueueDelay` (`.ActionManager` (`/Game/AdvancedTurnBasedTileToolkit/Core/BPFL_Singletons.GetActionManager2`)) 2.0))

(event `self.Activate`
  (params (`Target Unit` :type "/Game/AdvancedTurnBasedTileToolkit/Core/Units/BP_Unit Object Reference"))
  (bind _controllingunit (`self.ControllingUnit`))
  (bind _owningunit (`self.OwningUnit`))
  (`parent.Activate` `Target Unit`)
  (set `self.OldAlliedFactions` (`/Game/AdvancedTurnBasedTileToolkit/Core/Units/BP_Unit.AlliedFactions` _owningunit))
  (set `self.bOldAIControlled` (`/Game/AdvancedTurnBasedTileToolkit/Core/Units/BP_Unit.bAIControlled` _owningunit))
  (set `/Game/AdvancedTurnBasedTileToolkit/Core/Units/BP_Unit.AlliedFactions` (`/Game/AdvancedTurnBasedTileToolkit/Core/Units/BP_Unit.AlliedFactions` (select `bool` (`KismetSystemLibrary.IsValid` _controllingunit) :`false` (`/Game/AdvancedTurnBasedTileToolkit/Core/BP_TurnManager.ActiveUnit` (`.TurnManager` (`/Game/AdvancedTurnBasedTileToolkit/Core/BPFL_Singletons.GetTurnManager2`))) :`true` _controllingunit)) (`self.OwningUnit`))
  (set `/Game/AdvancedTurnBasedTileToolkit/Core/Units/BP_Unit.bAIControlled` true (`self.OwningUnit`))
  (goto _label))

(event `self.RunOnTurnEnd`
  (set `/Game/AdvancedTurnBasedTileToolkit/Core/Units/BP_Unit.AlliedFactions` (`self.OldAlliedFactions`) (`self.OwningUnit`))
  (set `/Game/AdvancedTurnBasedTileToolkit/Core/Units/BP_Unit.bAIControlled` (`self.bOldAIControlled`) (`self.OwningUnit`))
  (`self.Disable`))

(fn `UserConstructionScript`
  (`parent.UserConstructionScript`))