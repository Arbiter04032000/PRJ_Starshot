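; BP_Unit_2D_Hydra is a 2D hydra unit for the turn-based tile toolkit that gains heads as its health is modified and ends the game when killed.
; After any health change it survives, it increments its head count up to five and spawns a BP_Action_GrowHead_2D action, passing its hydra puppet and the new count.
; Its death runs the parent kill logic, then sets GameOver on the turn manager.
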(event `self.ModifyHealth`
  (params (Change :type "Float (single-precision)") (bAutoAnimate :type Boolean) (EndDelay :type "Float (single-precision)"))
  (`parent.ModifyHealth` Change bAutoAnimate EndDelay)
  (if (> (`self.CurrentHealth`) 0.0)
    (if (< (`self.Heads`) 5)
      (`/Engine/EditorBlueprintResources/StandardMacros.IncrementInt` (`self.Heads`)
        (:`  `
          (bind _asbp_2d_puppet_hydra (cast `/Game/AdvancedTurnBasedTileToolkit/Maps/2D/Units/BP_2D_Puppet_Hydra` (`self.Puppet`)))
          (`|SpawnActorFromClass` "/Game/AdvancedTurnBasedTileToolkit/Maps/2D/Actions/BP_Action_GrowHead_2D.BP_Action_GrowHead_2D_C" (`KismetMathLibrary.MakeTransform` (0.0 0.0 0.0)) "Undefined" "OverrideRootScale" null _asbp_2d_puppet_hydra (`self.Heads`) 0.5 "NewEnumerator0" null))))))

(event `self.KillUnit`
  (`parent.KillUnit`)
  (set `/Game/AdvancedTurnBasedTileToolkit/Core/BP_TurnManager.bGameOver` true (`.TurnManager` (`/Game/AdvancedTurnBasedTileToolkit/Core/BPFL_Singletons.GetTurnManager`))))

(fn `UserConstructionScript`
  (`parent.UserConstructionScript`))