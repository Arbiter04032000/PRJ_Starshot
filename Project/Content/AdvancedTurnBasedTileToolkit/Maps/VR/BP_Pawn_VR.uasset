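; VR pawn for the turn-based tile toolkit that turns motion controller pointing and trigger input into grid hover and click messages.
; On BeginPlay it sets floor tracking, waits for the turn manager, reports player readiness, then starts a looping client tick.
; The loop traces from the right arrow on the grid's path channel, drawing a debug line and sending hover hits.
; Both triggers reuse that right-arrow ray to send left-mouse press/release clicks.
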(event `ServerNotifyPlayerReady`
  (message `/Game/AdvancedTurnBasedTileToolkit/Core/BPI_GameState.NotifyPlayerReadyFromState` (`GameplayStatics.GetGameState`) (`GameplayStatics.GetPlayerController` 0)))

(event `self.ReceiveBeginPlay`
  (bind _returnvalue (`GameplayStatics.GetActorOfClass` "/Game/AdvancedTurnBasedTileToolkit/Core/Grid/BP_GridManager.BP_GridManager_C"))
  (set `self.GridManagerRef` _returnvalue)
  (`HeadMountedDisplayFunctionLibrary.SetTrackingOrigin` "Floor")
  (`/Game/AdvancedTurnBasedTileToolkit/Core/BPML_Utility.DelayWhile` (not (`/Game/AdvancedTurnBasedTileToolkit/Core/BPFL_Singletons.GetTurnManager`))
    (:`Continue`
      (`self.ServerNotifyPlayerReady`)
      (`self.ClientBeginClientTick`))))

(event `ClientBeginClientTick`
  (bind _arrowright (`self.ArrowRight`))
  (bind _returnvalue (`SceneComponent.K2_GetComponentLocation` _arrowright))
  (`/Game/AdvancedTurnBasedTileToolkit/Core/BPML_Utility.WhileLoop_Delayed` (`self.bRunClientTick`)
    (:`Loop Body`
      (bind _outhit (`KismetSystemLibrary.LineTraceSingle` :`Start` _returnvalue :`End` (+ _returnvalue (* (`SceneComponent.GetForwardVector` _arrowright) 20000.0)) :`TraceChannel` (`/Game/AdvancedTurnBasedTileToolkit/Core/Grid/BP_GridManager.PathTraceChannel` (`self.GridManagerRef`)) :`DrawDebugType` "ForOneFrame"))
      (if (`GameplayStatics.BreakHitResult` _outhit)
        (message `/Game/AdvancedTurnBasedTileToolkit/Core/BPI_GridInteraction.Hover` (`GameplayStatics.GetPlayerController` 0) (`.Location` (`GameplayStatics.BreakHitResult` _outhit)))))))

(event `InputAction|MotionControllerRightTrigger`
  (params (Key :type "Key Structure"))
  (bind _arrowright (`self.ArrowRight`))
  (bind _returnvalue (`SceneComponent.K2_GetComponentLocation` _arrowright))
  (:`Pressed`
    (set `self.bReleased` false :!label _label)
    (bind (_outhit _returnvalue_2) (`KismetSystemLibrary.LineTraceSingle` _returnvalue (+ _returnvalue (* (`SceneComponent.GetForwardVector` _arrowright) 20000.0)) (`/Game/AdvancedTurnBasedTileToolkit/Core/Grid/BP_GridManager.PathTraceChannel` (`self.GridManagerRef`)) :!label _label_2))
    (if _returnvalue_2
      (message `/Game/AdvancedTurnBasedTileToolkit/Core/BPI_GridInteraction.Click` (`GameplayStatics.GetPlayerController` 0) (`.Location` (`GameplayStatics.BreakHitResult` _outhit)) "LeftMouseButton" (`self.bReleased`) "NewEnumerator0")))
  (:`Released`
    (set `self.bReleased` true :!label _label_3)
    (goto _label_2)))

(event `InputAction|MotionControllerLeftTrigger`
  (params (Key :type "Key Structure"))
  (:`Pressed`
    (goto _label))
  (:`Released`
    (goto _label_3)))

(fn `UserConstructionScript`)