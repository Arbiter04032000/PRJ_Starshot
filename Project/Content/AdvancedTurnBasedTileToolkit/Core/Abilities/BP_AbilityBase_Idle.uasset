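; Idle ability for the turn-based tile toolkit that lets the active player select a unit on the grid.
; On a server interact, it acts only when a primary input is released over a valid tile.
; It looks up the clicked index in the grid manager's unit map and confirms the owner is the turn manager's active player.
; It then sends the select-actor message to that unit.
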(event `self.ServerInteract`
  (params (bValidTile :type Boolean) (ClickedIndex :type Integer) (Location :type "Vector Structure") (Key :type "Key Structure") (bReleased :type Boolean) (ClickType :type "/Game/AdvancedTurnBasedTileToolkit/Core/Grid/EClickType Enum" :default "NewEnumerator0") (CallingPc :type "/Game/AdvancedTurnBasedTileToolkit/Core/BP_PlayerController_ATBTT Object Reference"))
  (if bValidTile
    (if bReleased
      (switch `/Game/AdvancedTurnBasedTileToolkit/Core/Grid/EClickType` "NewEnumerator0"
        (:`NewEnumerator0`
          (if (`.ReturnValue` (`BlueprintMapLibrary.Map_Find` (`/Game/AdvancedTurnBasedTileToolkit/Core/Grid/BP_GridManager.GridUnits` (`self.GridManagerRef`)) ClickedIndex))
            (if (== (`/Game/AdvancedTurnBasedTileToolkit/Core/BP_TurnManager.ActivePlayer` (`.TurnManager` (`/Game/AdvancedTurnBasedTileToolkit/Core/BPFL_Singletons.GetTurnManager`))) (`self.GetOwner`))
              (message `/Game/AdvancedTurnBasedTileToolkit/Core/BPI_Initiative.SelectActor` (`BlueprintMapLibrary.Map_Find` (`/Game/AdvancedTurnBasedTileToolkit/Core/Grid/BP_GridManager.GridUnits` (`self.GridManagerRef`)) (`self.ClickedIndex`))))))))))

(fn `UserConstructionScript`
  (`parent.UserConstructionScript`))