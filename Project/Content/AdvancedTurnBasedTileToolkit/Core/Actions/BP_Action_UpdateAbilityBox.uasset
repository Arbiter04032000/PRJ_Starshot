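; BP_Action_UpdateAbilityBox is a turn-based toolkit action that refreshes the ability box in the HUD.
; On BeginPlay, the authority snapshots charges, cooldowns and ability references from a valid AbilitySystem.
; When played, it passes that snapshot to the first player controller's HUD widget, showing the box only if owned by the client and the AbilitySystem is valid.
; The action ends immediately, even if the HUD cast fails.
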(event `self.ReceiveBeginPlay`
  (bind _abilitysystem (`self.AbilitySystem`))
  (`parent.ReceiveBeginPlay`)
  (`/Engine/EditorBlueprintResources/ActorMacros.Switch Has Authority`
    (:`Authority`
      (`/Engine/EditorBlueprintResources/StandardMacros.IsValid` _abilitysystem
        (:`Is Valid`
          (set `self.Charges` (`/Game/AdvancedTurnBasedTileToolkit/Core/Units/BP_AbilitySystem.Charges` _abilitysystem))
          (set `self.Cooldowns` (`/Game/AdvancedTurnBasedTileToolkit/Core/Units/BP_AbilitySystem.Cooldowns` _abilitysystem))
          (set `self.Abilities` (`/Game/AdvancedTurnBasedTileToolkit/Core/Units/BP_AbilitySystem.AbilityRefs` _abilitysystem)))))))

(event `self.PlayAction`
  (bind _asbp_hud_atbtt (cast `/Game/AdvancedTurnBasedTileToolkit/Core/UI/BP_HUD_ATBTT` (`PlayerController.GetHUD` (`GameplayStatics.GetPlayerController` 0)))
    (:`then`
      (bind _bownedbyclient (`self.IsOwnedByClient`))
      (`/Game/AdvancedTurnBasedTileToolkit/Core/UI/WBP_AbilityBox.RefreshAbilityBox` (`/Game/AdvancedTurnBasedTileToolkit/Core/UI/WBP_ATBTT.WBP_AbilityBox` (`/Game/AdvancedTurnBasedTileToolkit/Core/UI/BP_HUD_ATBTT.WbpAtbttRef` _asbp_hud_atbtt)) (and _bownedbyclient (`KismetSystemLibrary.IsValid` (`self.AbilitySystem`))) (`self.Abilities`) (`self.Charges`) (`self.Cooldowns`))
      (`self.EndAction` true))
    (:`CastFailed`
      (`self.EndAction` true))))

(fn `UserConstructionScript`
  (`parent.UserConstructionScript`))