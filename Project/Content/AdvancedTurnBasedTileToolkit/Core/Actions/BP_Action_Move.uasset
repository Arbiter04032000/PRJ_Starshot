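; Turn-based action that animates an actor moving along a tile path, then ends the action.
; PlayAction loads MovePath into a child-actor spline and steps along it in a delayed loop, with optional acceleration and speed scaled by tile size.
; Each step updates animation speed, yaw and position, optionally line-tracing for ground height.
; An optional target marker at the destination shows only for the owning client and hides on completion.
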(event `self.PlayAction`
  (bind _movedactor (`self.MovedActor`))
  (bind _currentspeed (`self.CurrentSpeed`))
  (bind (_returnvalue_x _returnvalue_y _returnvalue_z) (`KismetMathLibrary.BreakVector` (`self.GetActorScale3D` _movedactor)))
  (bind _returnvalue (`SplineComponent.GetLocationAtDistanceAlongSpline` (`/Game/AdvancedTurnBasedTileToolkit/Core/Units/BP_PathSpline.Spline` (`self.PathSplineRef`)) (`self.CurrentSplineDistance`) "World"))
  (bind ___ (`/Game/AdvancedTurnBasedTileToolkit/Core/Grid/BP_GridManager.ConvertFromGridToWorld` (`self.GridManagerRef`) _returnvalue))
  (`/Game/AdvancedTurnBasedTileToolkit/Core/BPFL_Singletons.ClearMarkers`)
  (set `self.GridManagerRef` (`.GridManager` (`/Game/AdvancedTurnBasedTileToolkit/Core/BPFL_Singletons.GetGridManager`)))
  (bind _asbp_path_spline (cast `/Game/AdvancedTurnBasedTileToolkit/Core/Units/BP_PathSpline` (`ChildActorComponent.ChildActor` (`self.PathSpline`)))
    (:`then`
      (set `self.PathSplineRef` _asbp_path_spline)
      (`self.ShowTargetMarkerIfAllowed`)
      (`SplineComponent.SetSplinePoints` (`/Game/AdvancedTurnBasedTileToolkit/Core/Units/BP_PathSpline.Spline` (`self.PathSplineRef`)) (`self.MovePath`) "World" true)
      (bind _offset (message `/Game/AdvancedTurnBasedTileToolkit/Core/BPI_Puppet.GetPuppetOffset` (`self.MovedActor`)))
      (set `self.Offset` _offset)
      (set `self.CurrentSplineDistance` 0.0)
      (if (not (`self.bAccelerate`))
        (set `self.CurrentSpeed` (`self.MaxSpeed`)))
      (`/Game/AdvancedTurnBasedTileToolkit/Core/BPML_Utility.WhileLoop_Delayed` (< (`self.CurrentSplineDistance`) (`SplineComponent.GetSplineLength` (`/Game/AdvancedTurnBasedTileToolkit/Core/Units/BP_PathSpline.Spline` (`self.PathSplineRef`))))
        (:`Loop Body`
          (message `/Game/AdvancedTurnBasedTileToolkit/Core/BPI_Puppet.AnimateMovement` _movedactor (/ (`self.CurrentSpeed`) _returnvalue_z))
          (if (> (`self.MaxSpeed`) _currentspeed)
            (set `self.CurrentSpeed` (+ _currentspeed (`self.Acceleration`))))
          (set `self.CurrentSplineDistance` (`KismetMathLibrary.FMin` (+ (`self.CurrentSplineDistance`) (* (* (* (`GameplayStatics.GetWorldDeltaSeconds`) (`self.CurrentSpeed`)) (/ (`/Game/AdvancedTurnBasedTileToolkit/Core/Grid/BP_GridManager.TileXSize` (`.GridManager` (`/Game/AdvancedTurnBasedTileToolkit/Core/BPFL_Singletons.GetGridManager`))) 200.0)) (`self.SpeedModifier`))) (`SplineComponent.GetSplineLength` (`/Game/AdvancedTurnBasedTileToolkit/Core/Units/BP_PathSpline.Spline` (`self.PathSplineRef`)))))
          (`self.K2_SetActorRelativeRotation` (`self.MovedActor`) (`KismetMathLibrary.MakeRotator` 0.0 0.0 (.yaw (`SplineComponent.GetRotationAtDistanceAlongSpline` (`/Game/AdvancedTurnBasedTileToolkit/Core/Units/BP_PathSpline.Spline` (`self.PathSplineRef`)) (`self.CurrentSplineDistance`) "World"))) false false)
          (if (`self.bTraceForGround`)
            (bind _outhit (`KismetSystemLibrary.LineTraceSingle` ___ (- ___ (* (`SceneComponent.GetUpVector` (`Actor.RootComponent` (`self.MovedActor`))) -200.0)) "TraceTypeQuery1"))
            (`self.K2_SetActorLocation` (`self.MovedActor`) (+ (`self.Offset`) (`.ImpactPoint` (`GameplayStatics.BreakHitResult` _outhit))) false false)
            (else
              (`self.K2_SetActorLocation` (`self.MovedActor`) (+ _returnvalue (`self.Offset`)) false false))))
        (:`Completed`
          (bind _gridui (message `/Game/AdvancedTurnBasedTileToolkit/Core/BPI_Ability.GetGridUi` (`GameplayStatics.GetPlayerController` 0) (`self.GridUIClassOverride`)))
          (`/Game/AdvancedTurnBasedTileToolkit/Core/GridUI/BP_GridUI.DisplayTargetMarker` _gridui (0.0 0.0 0.0) false)
          (message `/Game/AdvancedTurnBasedTileToolkit/Core/BPI_Puppet.AnimateMovement` (`self.MovedActor`) 0.0)
          (`self.EndAction` true))))
    (:`CastFailed`
      (`self.EndAction` true))))

(event `self.ReceiveDestroyed`
  (`self.K2_DestroyActor` (`self.PathSplineRef`)))

(fn `ShowTargetMarkerIfAllowed`
  (returns (bMarkerIsShown :type Boolean))
  (bind _movepath (`self.MovePath`))
  (if (`self.bShowTargetMarker`)
    (bind _bownedbyclient (`self.IsOwnedByClient`))
    (bind _gridui (message `/Game/AdvancedTurnBasedTileToolkit/Core/BPI_Ability.GetGridUi` (`GameplayStatics.GetPlayerController` 0) (`self.GridUIClassOverride`)))
    (`/Game/AdvancedTurnBasedTileToolkit/Core/GridUI/BP_GridUI.DisplayTargetMarker` _gridui (`|GetArrayItem` _movepath (`KismetArrayLibrary.Array_LastIndex` _movepath)) _bownedbyclient)
    (return _bownedbyclient)
    (else
      (return false))))

(fn `UserConstructionScript`
  (`parent.UserConstructionScript`))