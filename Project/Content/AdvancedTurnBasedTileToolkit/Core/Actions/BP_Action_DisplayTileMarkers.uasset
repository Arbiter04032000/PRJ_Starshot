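; Queued action in the turn-based tile toolkit that displays tile markers of a given type at a set of tile locations through the grid UI.
; In networked games, the authority adds the locations to the action manager's vector array messages during setup.
; Play reads the next message, or uses the local locations in standalone, spawns the markers and ends immediately.
; Skipping still advances the message to keep the queue aligned.
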(event `self.SetupAction`
  (if (and (not (`KismetSystemLibrary.IsStandalone`)) (`self.HasAuthority`))
    (`/Engine/EditorBlueprintResources/StandardMacros.IsValid` (`self.ManagerOverride`)
      (:`Is Valid`
        (message `/Game/AdvancedTurnBasedTileToolkit/Core/BPI_Action.AddToVectorArrayToManager` (`self.ManagerOverride`) (`self.TileLocations`)))
      (:`Is Not Valid`
        (message `/Game/AdvancedTurnBasedTileToolkit/Core/BPI_Action.AddToVectorArrayToManager` (`.ActionManager` (`/Game/AdvancedTurnBasedTileToolkit/Core/BPFL_Singletons.GetActionManager`)) (`self.TileLocations`))))))

(event `self.PlayAction`
  (bind _gridui (message `/Game/AdvancedTurnBasedTileToolkit/Core/BPI_Ability.GetGridUi` (`GameplayStatics.GetPlayerController` 0) (`self.GridUIClassOverride`)))
  (if (`KismetSystemLibrary.IsStandalone`)
    (`/Game/AdvancedTurnBasedTileToolkit/Core/GridUI/BP_GridUI.SpawnTileMarkers` _gridui (`self.MarkerType`) (`self.TileLocations`))
    (else
      (bind _vectors (message `/Game/AdvancedTurnBasedTileToolkit/Core/BPI_Action.AdvanceAndGetNextVectorArrayToManager` (`self.ManagerOverride`)))
      (`/Game/AdvancedTurnBasedTileToolkit/Core/GridUI/BP_GridUI.SpawnTileMarkers` _gridui (`self.MarkerType`) _vectors)))
  (`self.EndAction` true))

(event `self.RunOnSkipAction`
  (if (not (`KismetSystemLibrary.IsStandalone`))
    (message `/Game/AdvancedTurnBasedTileToolkit/Core/BPI_Action.AdvanceAndGetNextVectorArrayToManager` (`self.ManagerOverride`)))
  (`parent.RunOnSkipAction`))

(fn `UserConstructionScript`
  (`parent.UserConstructionScript`))