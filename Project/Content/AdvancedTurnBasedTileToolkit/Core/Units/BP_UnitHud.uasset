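; BP_UnitHud is a widget component that serves as a unit's HUD, showing its health bar and status effects.
; On BeginPlay it passes itself to its user widget as owner component, then forwards health fill and status effect changes through message calls.
; It also toggles widget visibility, while GetGunMuzzle and GetPuppetCenter are stubs returning invalid and zero values.
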(event `self.ReceiveBeginPlay`
  (message `/Game/AdvancedTurnBasedTileToolkit/Core/Units/BPI_UnitHUD.SetOwnerComponent` (`self.GetUserWidgetObject`) self))

(event `/Game/AdvancedTurnBasedTileToolkit/Core/Units/BPI_UnitHUD.SetHealthBarFill`
  (params (PercentFill :type "Float (single-precision)"))
  (message `/Game/AdvancedTurnBasedTileToolkit/Core/Units/BPI_UnitHUD.SetHealthBarFill` (`self.GetUserWidgetObject`) PercentFill))

(event `/Game/AdvancedTurnBasedTileToolkit/Core/Units/BPI_UnitHUD.DisplayStatusEffect`
  (params (bRemove :type Boolean) (StatusEffect :type "/Game/AdvancedTurnBasedTileToolkit/Core/Abilities/BP_StatusEffect Class Reference"))
  (message `/Game/AdvancedTurnBasedTileToolkit/Core/Units/BPI_UnitHUD.DisplayStatusEffect` (`self.GetUserWidgetObject`) bRemove StatusEffect))

(event `/Game/AdvancedTurnBasedTileToolkit/Core/Units/BPI_UnitHUD.SetHudVisibility`
  (params (bVisible :type Boolean))
  (`Widget.SetVisibility` (`self.GetUserWidgetObject`) (select `bool` bVisible :`false` "Hidden" :`true` "Visible" :!type "ESlateVisibility Enum")))

(fn `GetGunMuzzle`
  (returns (bValid :type Boolean) (GunComponent :type "StaticMeshComponent Object Reference") (MuzzleTransform :type "Transform Structure"))
  (return false null))

(fn `GetPuppetCenter`
  (returns (Location :type "Vector Structure"))
  (return (0.0 0.0 0.0)))