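; Unit component for the tile toolkit's stealth system that keeps a unit unaware until it sees or hears activity on the grid.
; On BeginPlay it waits for the grid manager's BP_StealthSystem to finish setup, then binds to its noise and sight-check events.
; Noise wakes it by tile range; sight also requires front-arc facing, visibility and, with a cover system, an unblocked trace.
; Waking applies a Woke status effect and moves the unit in initiative.
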(event `self.ReceiveBeginPlay`
  (bind (_bvalid _gridmanager) (`/Game/AdvancedTurnBasedTileToolkit/Core/BPFL_Singletons.GetGridManager`))
  (bind _asbp_unit (cast `/Game/AdvancedTurnBasedTileToolkit/Core/Units/BP_Unit` (`self.GetOwner`))
    (:`then`
      (set `self.OwningUnit` _asbp_unit)
      (if _bvalid
        (bind _output_get (set `self.GridManagerRef` _gridmanager))
        (bind _returnvalue (`Actor.GetComponentByClass` _output_get "/Game/AdvancedTurnBasedTileToolkit/Core/Grid/BP_StealthSystem.BP_StealthSystem_C"))
        (if (`KismetSystemLibrary.IsValid` _returnvalue)
          (if (`/Game/AdvancedTurnBasedTileToolkit/Core/Grid/BP_StealthSystem.bSetupDone` _returnvalue) :!label _label
            (if (`self.bUnaware`)
              (add `/Game/AdvancedTurnBasedTileToolkit/Core/Grid/BP_StealthSystem.OnCheckIfSeen` _returnvalue (delegate `Spot`))
              (add `/Game/AdvancedTurnBasedTileToolkit/Core/Grid/BP_StealthSystem.OnMakeNoise` _returnvalue (delegate `Listen`)))
            (else
              (`KismetSystemLibrary.Delay` 0.0)
              (goto _label)))
          (else
            (`KismetSystemLibrary.PrintString` "WARNING: Unit has stealth system, but Grid Manager does not." true true (struct :`R` 1.0 :`G` 1.0 :`A` 1.0))))))
    (:`CastFailed`
      (`KismetSystemLibrary.PrintString` "WARNING: BP_Unit_StealthSystem added to \nactor other than BP_Unit" true true (struct :`R` 1.0 :`G` 1.0 :`A` 1.0)))))

(event `Listen`
  (params (Index :type Integer) (Range :type Integer))
  (if (`self.bUnaware`)
    (if (>= Range (`/Game/AdvancedTurnBasedTileToolkit/Core/Grid/BP_GridManager.FindDistanceIinTilesBetweenIndexes` (`self.GridManagerRef`) Index (`/Game/AdvancedTurnBasedTileToolkit/Core/Units/BP_Unit.GridIndex` (`self.OwningUnit`)) false))
      (`self.Wake`))))

(event `Wake`
  (bind _returnvalue (`Actor.GetComponentByClass` (`self.OwningUnit`) "/Game/AdvancedTurnBasedTileToolkit/Core/Units/BP_AbilitySystem.BP_AbilitySystem_C"))
  (if (`self.bUnaware`)
    (set `self.bUnaware` false)
    (if (`BlueprintMapLibrary.Map_Contains` (`/Game/AdvancedTurnBasedTileToolkit/Core/Grid/BP_GridManager.GridUnits` (`self.GridManagerRef`)) (`/Game/AdvancedTurnBasedTileToolkit/Core/Units/BP_Unit.GridIndex` (`self.OwningUnit`)))
      (if (`KismetSystemLibrary.IsValid` _returnvalue)
        (`/Game/AdvancedTurnBasedTileToolkit/Core/Units/BP_AbilitySystem.AddStatusEffect` _returnvalue "/Game/AdvancedTurnBasedTileToolkit/Core/Abilities/BP_StatusEffect_Woke.BP_StatusEffect_Woke_C"))
      (`/Game/AdvancedTurnBasedTileToolkit/Core/BP_TurnManager.MoveActorInInitiative` (`.TurnManager` (`/Game/AdvancedTurnBasedTileToolkit/Core/BPFL_Singletons.GetTurnManager`)) (`self.InitiativeOnWake`) (`self.OwningUnit`)))))

(event `Spot`
  (params (Index :type Integer) (Range :type Integer))
  (bind _gridmanagerref (`self.GridManagerRef`))
  (bind _gridlocations (`/Game/AdvancedTurnBasedTileToolkit/Core/Grid/BP_GridManager.GridLocations` (`self.GridManagerRef`)))
  (bind _distance (`/Game/AdvancedTurnBasedTileToolkit/Core/Grid/BP_GridManager.FindDistanceIinTilesBetweenIndexes` (`self.GridManagerRef`) (`/Game/AdvancedTurnBasedTileToolkit/Core/Units/BP_Unit.GridIndex` (`self.OwningUnit`)) Index false))
  (bind (_returnvalue_roll _returnvalue_pitch _returnvalue_yaw) (`KismetMathLibrary.BreakRotator` (`KismetMathLibrary.NormalizedDeltaRotator` (`Actor.K2_GetActorRotation` (`self.OwningUnit`)) (`KismetMathLibrary.FindLookAtRotation` (`BlueprintMapLibrary.Map_Find` _gridlocations (`/Game/AdvancedTurnBasedTileToolkit/Core/Units/BP_Unit.GridIndex` (`self.OwningUnit`))) (`BlueprintMapLibrary.Map_Find` _gridlocations Index)))))
  (bind _returnvalue (`KismetMathLibrary.Abs` _returnvalue_yaw))
  (if (`self.bUnaware`)
    (if (`KismetMathLibrary.BooleanNAND` (< _returnvalue 269.0) (> _returnvalue 91.0))
      (if (>= Range _distance)
        (bind _bvisible (`/Game/AdvancedTurnBasedTileToolkit/Core/Grid/BP_GridManager.CheckIfTileIsVisibleFromOtherTile` (`self.GridManagerRef`) (`/Game/AdvancedTurnBasedTileToolkit/Core/Units/BP_Unit.GridIndex` (`self.OwningUnit`)) Index (* _distance (`/Game/AdvancedTurnBasedTileToolkit/Core/Grid/BP_GridManager.TileXSize` (`self.GridManagerRef`))) 0 true false))
        (if _bvisible
          (if (`KismetSystemLibrary.IsValid` (`Actor.GetComponentByClass` (`self.GridManagerRef`) "/Game/AdvancedTurnBasedTileToolkit/Core/Grid/BP_CoverSystem.BP_CoverSystem_C"))
            (bind _hit (`/Game/AdvancedTurnBasedTileToolkit/Core/Grid/BP_GridManager.TraceOnGrid` _gridmanagerref (`/Game/AdvancedTurnBasedTileToolkit/Core/Units/BP_Unit.GridIndex` (`self.OwningUnit`)) Index "TraceTypeQuery5" "None" (`/Game/AdvancedTurnBasedTileToolkit/Core/Grid/BP_GridManager.VisibilityTraceHeight` _gridmanagerref)))
            (if (not _hit)
              (`self.Wake` :!label _label_2))
            (else
              (goto _label_2))))))))