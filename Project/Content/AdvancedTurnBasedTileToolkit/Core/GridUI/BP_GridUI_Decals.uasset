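; BP_GridUI_Decals is a Grid UI Blueprint in the Advanced Turn Based Tile Toolkit that shows tile markers as decals.
; SpawnTileMarkers looks up the default decal material for a marker type and spawns decals with it at the given locations.
; ClearTileMarkers clears decals by that same material, so the material serves as the key for each marker type.
; The event graph holds no active logic.
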(fn `ClearTileMarkers`
  (params (MarkerType :type "/Game/AdvancedTurnBasedTileToolkit/Core/ETileMarkerType Enum" :default "NewEnumerator0"))
  (`self.ClearSpecifiedDecals` (`self.GetDefaultMarkerDecal` MarkerType))
  (return))

(fn `SpawnTileMarkers`
  (params (MarkerType :type "/Game/AdvancedTurnBasedTileToolkit/Core/ETileMarkerType Enum" :default "NewEnumerator0") (Locations :type "Array of Vector Structure (by ref)"))
  (`self.Spawn Decals at Locations` Locations (`self.GetDefaultMarkerDecal` MarkerType))
  (return))

(fn `UserConstructionScript`
  (`parent.UserConstructionScript`))