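; FL_ParseSkimmer is a string-parsing function library that skims item command strings for the variable names they reference.
; ItemSkimTypes splits input on commas, runs each piece through Breaker, and collects map keys where the first keyword is Add or Replace.
; Breaker tokenizes a piece, moving tokens containing "(" into a name-to-argument map and returning it with the remaining keywords.
; ItemSkimAllVars is an empty stub.
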(fn `Breaker`
  (params (input :type String))
  (returns (keys :type "Array of String") (keyvar :type "Map of String to String"))
  (locals (purgeindices :type "Array of Integer") (keyArray :type "Array of String") (keyMap :type "Map of String to String"))
  (bind _output_get (set `local.keyArray` (`KismetStringLibrary.ParseIntoArray` input)))
  (for (_array_element _array_index) _output_get
    (if (`KismetStringLibrary.Contains` _array_element "(")
      (bind _returnvalue (`KismetStringLibrary.ParseIntoArray` _array_element "("))
      (`BlueprintMapLibrary.Map_Add` (`local.keyMap`) (`|GetArrayItem` _returnvalue) (`KismetStringLibrary.LeftChop` (`|GetArrayItem` _returnvalue 1)))
      (`KismetArrayLibrary.Array_Add` (`local.purgeindices`) _array_index)))
  (for _array_element_2 (`local.purgeindices`)
    (`KismetArrayLibrary.Array_Remove` (`local.keyArray`) _array_element_2))
  (return (`local.keyArray`) (`local.keyMap`)))

(fn `Item Skim All Vars`
  (params (input :type String)))

(fn `ItemSkim_Types`
  (params (input :type String))
  (returns (output :type "Array of String"))
  (locals (keycache :type "Array of String"))
  (bind _keycache (`local.keycache`))
  (for _array_element (`KismetStringLibrary.ParseIntoArray` input ",")
    (bind (_keys _keyvar) (`self.Breaker` _array_element))
    (switch `string` (`|GetArrayItem` _keys)
      (:`add`
        (bind _keys_2 (`BlueprintMapLibrary.Map_Keys` _keyvar))
        (`KismetArrayLibrary.Array_Append` _keycache _keys_2))
      (:`replace`
        (bind _keys_3 (`BlueprintMapLibrary.Map_Keys` _keyvar))
        (`KismetArrayLibrary.Array_Append` _keycache _keys_3))))
  (return (`local.keycache`)))