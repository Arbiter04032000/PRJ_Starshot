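; Base pawn for game pieces in the Starshot strategy game, handling mouse hover highlighting and left-click selection.
; Hover or selection turns on the model's custom depth rendering.
; Clicks toggle selection through SelectedPawn on GM_StarshotStrategyBP, deselecting any other pawn first, but self-deselection leaves that reference set.
; AltClickEvent is an empty stub; right-click handling and construction-time mesh, color and rotation randomization are disconnected.
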(event `self.ReceiveActorBeginCursorOver`
  (`self.OverlapEvent` true))

(event `self.ReceiveActorEndCursorOver`
  (`self.OverlapEvent` false))

(event `self.ReceiveActorOnClicked`
  (params (ButtonPressed :type "Key Structure"))
  (if (== ButtonPressed "LeftMouseButton")
    (`self.ClickEvent`)))

(event `OverlapEvent`
  (params (IsOverlapping :type Boolean))
  (`PrimitiveComponent.SetRenderCustomDepth` (`self.Model`) (or IsOverlapping (`self.IsSelected`))))

(event `ClickEvent`
  (bind _asgm_starshot_strategy_bp (cast `/Game/Blueprints/GameSettings/GM_StarshotStrategyBP` (`GameplayStatics.GetGameMode`)))
  (bind _selectedpawn (`/Game/Blueprints/GameSettings/GM_StarshotStrategyBP.SelectedPawn` _asgm_starshot_strategy_bp))
  (if (not (`KismetSystemLibrary.IsValid` _selectedpawn))
    (set `self.IsSelected` true :!label _label)
    (`self.OverlapEvent` false)
    (set `/Game/Blueprints/GameSettings/GM_StarshotStrategyBP.SelectedPawn` self _asgm_starshot_strategy_bp)
    (`KismetSystemLibrary.PrintString` "Set selected pawn")
    (elif (!= _selectedpawn self)
      (bind _output_get (set `/Game/Blueprints/GamePieces/Pawn_BaseType.IsSelected` false _selectedpawn))
      (`self.OverlapEvent` _selectedpawn _output_get)
      (goto _label)
      (else
        (set `self.IsSelected` false)
        (`self.OverlapEvent` false)))))

(event `AltClickEvent`
  (params (HitActor :type "Actor Object Reference") (IsPawn :type Boolean) (Enum_PawnType :type "/Game/Blueprints/GamePieces/Enum_PawnClass Enum" :default "NewEnumerator0")))

(fn `UserConstructionScript`)