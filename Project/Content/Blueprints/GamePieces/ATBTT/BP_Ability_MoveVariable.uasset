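; BP_Ability_MoveVariable is a unit movement ability that works out how much movement its owning unit can make.
; It overrides UpdateAttributes, calling the parent and then setting PossibleMove to the unit's CurrentAP divided by its Move attribute.
; Both MoveCostType options, per-move attribute value and pathfinding cost, currently share that same calculation.
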(event `self.UpdateAttributes`
  (bind _owningunit (`self.OwningUnit`))
  (`parent.UpdateAttributes`)
  (switch `/Game/AdvancedTurnBasedTileToolkit/Core/Abilities/EMoveCost` (`self.MoveCostType`)
    (:`NewEnumerator2`
      _)
    (:`NewEnumerator3`
      _))
  (set `self.PossibleMove` (/ (`/Game/AdvancedTurnBasedTileToolkit/Core/Units/BP_Unit.CurrentAP` _owningunit) (`/Game/AdvancedTurnBasedTileToolkit/Core/Units/BP_Unit.Move` _owningunit))))

(fn `UserConstructionScript`
  (`parent.UserConstructionScript`))