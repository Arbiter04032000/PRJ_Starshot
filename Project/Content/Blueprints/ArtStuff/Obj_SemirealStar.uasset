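; Semi-real star actor that pairs a visible Star component with a directional light, both driven by shared settings.
; The construction script offsets the star along local negative X by StarDistance and scales it uniformly by StarScale.
; Colour feeds both the star materials' "Light" parameter and the light colour, while Intensity sets only the light's brightness.
; It has no active runtime logic.
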(fn `UserConstructionScript`
  (bind _star (`self.Star`))
  (bind _colour (`self.Colour`))
  (bind _directionallight (`self.DirectionalLight`))
  (`SceneComponent.K2_SetRelativeTransform` _star (`KismetMathLibrary.MakeTransform` (`KismetMathLibrary.MakeVector` (* (`self.StarDistance`) -1.0)) (struct) (`KismetMathLibrary.Conv_DoubleToVector` (`self.StarScale`))) false false)
  (`MeshComponent.SetVectorParameterValueOnMaterials` _star "Light" (`KismetMathLibrary.Conv_LinearColorToVector` _colour))
  (`LightComponent.SetLightColor` _directionallight _colour true)
  (`LightComponent.SetIntensity` _directionallight (`self.Intensity`)))