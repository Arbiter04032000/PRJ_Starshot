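; Gas giant prop actor with an optional planetary ring, configured entirely in the construction script.
; RingEnabled assigns a plane mesh to the Ring component or clears it.
; The ring material's Color parameter comes from either a fixed Colour or RingCurve sampled at CurveTime, boosted to a high intensity.
; The event graph holds only disabled default events, so no runtime logic runs.
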(fn `UserConstructionScript`
  (bind _ring (`self.Ring`))
  (`parent.UserConstructionScript`)
  (`StaticMeshComponent.SetStaticMesh` _ring (select `bool` (`self.RingEnabled`) :`true` "/Game/StarterContent/Shapes/Shape_Plane.Shape_Plane" :!type "StaticMesh Object Reference"))
  (`MeshComponent.SetVectorParameterValueOnMaterials` _ring "Color" (* (`KismetMathLibrary.Conv_LinearColorToVector` (select `bool` (`self.UseCurve`) :`false` (`self.Colour`) :`true` (`CurveLinearColor.GetLinearColorValue` (`self.RingCurve`) (`self.CurveTime`)))) 10.0)))