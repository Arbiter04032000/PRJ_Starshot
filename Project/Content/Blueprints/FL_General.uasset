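; General function library of shared helpers for array and map edits and for reading dialogue-style text and response data.
; The array helper counts and locates every match of a Name, overwriting each match with a placeholder, while the map helper re-adds a String-to-Bool entry after removing it.
; Two BreakByID lookups split rows from the text and response index DataTables into individual fields, printing a red error when an ID is missing.
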(fn `BreakByID_Responses`
  (params (ID :type Name))
  (returns (ID_r :type Name) (Struct :type "/Game/Assets/Datatables/TextData/Struct_ResponseData Structure") (Text :type Text) (TextDataID :type Name) (ReqString :type String) (EventString :type String) (NextPart :type Name) (TimeToNextPart :type Integer) (PostBattleMap :type "Map of /Game/Blueprints/GameSettings/Struct_PostBattleKey Structure to Name") (RewardOnce :type Boolean) (UsesContinuity :type Boolean) (ContinuitySettings :type "/Game/Assets/Datatables/TextData/Struct_ContinuityToUse Structure") (`Pass-Over` :type Boolean))
  (bind _returnvalue (`|GetDataTableRow` "/Game/Assets/Datatables/TextData/DTRD_Index.DTRD_Index" ID)
    (:`then`
      (bind (_text _textdataid _reqstring _eventstring _nextpart _timetonextpart _postbattlemap _rewardonce _usescontinuity _continuitysettings _pass_over) (break `/Game/Assets/Datatables/TextData/Struct_ResponseData` _returnvalue))
      (return ID _returnvalue _text _textdataid _reqstring _eventstring _nextpart _timetonextpart _postbattlemap _rewardonce _usescontinuity _continuitysettings _pass_over))
    (:`RowNotFound`
      (`KismetSystemLibrary.PrintText` null (`|FormatText` "ResponseData Row of ID [ {ID} ] not found in table [ Index ]" ID) true true (struct :`R` 1.0 :`A` 1.0)))))

(fn `BreakByID_Text`
  (params (ID :type Name))
  (returns (ID_r :type Name) (Text :type Text) (Responses :type "Array of Name") (Type :type Byte) (`IsRandom?` :type Boolean) (Rarity :type "/Game/Assets/Datatables/Enum_Rarity Enum") (`OnlyOnce?` :type Boolean) (Continuity :type "/Game/Assets/Datatables/TextData/Struct_ContinuityToUse Structure"))
  (bind _returnvalue (`|GetDataTableRow` "/Game/Assets/Datatables/TextData/DTTD_Index.DTTD_Index" ID)
    (:`then`
      (bind (_text _responses _type _israndom_ _rarity _onlyonce_ _continuity) (break `/Game/Assets/Datatables/TextData/Struct_TextData` _returnvalue))
      (return ID _text _responses _type _israndom_ _rarity _onlyonce_ _continuity))
    (:`RowNotFound`
      (`KismetSystemLibrary.PrintText` null (`|FormatText` "TextData Row of ID [ {ID} ] not found in table [ Index ]" ID) true true (struct :`R` 1.0 :`A` 1.0)))))

(fn `Delete and Add Entry (Str B)`
  (params (MapToMod :type "Map of String to Boolean") (String :type String) (Bool :type Boolean))
  (returns (output :type "Map of String to Boolean"))
  (locals (NewLocalVar_0 :type "Map of String to Boolean"))
  (`KismetSystemLibrary.PrintText` null (`|FormatText` "Attempting removal of {s}" String))
  (bind _output_get (set `local.NewLocalVar_0` MapToMod))
  (bind _returnvalue (`BlueprintMapLibrary.Map_Remove` _output_get String))
  (if (not _returnvalue)
    (`KismetSystemLibrary.PrintString` null "Map location missing, try again?"))
  (`BlueprintMapLibrary.Map_Add` _output_get String Bool)
  (return (`local.NewLocalVar_0`)))

(fn `Find All In Array (Name)`
  (params (in :type "Array of Name") (toFind :type Name))
  (returns (`out#` :type Integer) (locs :type "Array of Integer"))
  (locals (counter :type Integer) (locations :type "Array of Integer") (cache :type "Array of Name"))
  (bind _output_get (set `local.cache` in))
  (for (_array_element _array_index) _output_get
    (if (== toFind _array_element)
      (`/Engine/EditorBlueprintResources/StandardMacros.IncrementInt` (`local.counter`)
        (:`  `
          (`KismetArrayLibrary.Array_Add` (`local.locations`) _array_index)
          (`|VariableSetRef` (`|GetArrayItem` _output_get _array_index) "fl_holdingvar_pleaseneverusethisvaluekthx")))))
  (return (`local.counter`) (`local.locations`)))