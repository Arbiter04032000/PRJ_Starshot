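; GM_StarshotStoryBP, apparently the story-mode game mode for Starshot, provides a shared, pausable game timer.
; On BeginPlay it starts a looping timer, stores its handle, then calls MSwitchAndStart on the GI_Starshot game instance.
; Each tick of that timer prints a log-only debug string and fires TimerDispatch for any listeners.
; PauseEvent and UnpauseEvent pause and resume the timer through the stored handle.
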(event `self.ReceiveBeginPlay`
  (bind _returnvalue (`KismetSystemLibrary.K2_SetTimerDelegate` (delegate `TimerEvent`) (`self.TimerTime`) true))
  (set `self.TimerHandle` _returnvalue)
  (bind _asgi_starshot (cast `/Game/Blueprints/GameSettings/GI_Starshot` (`GameplayStatics.GetGameInstance`)))
  (`/Game/Blueprints/GameSettings/GI_Starshot.mSwitchAndStart` _asgi_starshot "NewEnumerator0"))

(event `TimerEvent`
  (`KismetSystemLibrary.PrintString` "TimerCall" false true (struct :`G` 0.66 :`B` 1.0 :`A` 1.0) 1.0)
  (`self.TimerDispatch`))

(event `UnpauseEvent`
  (`KismetSystemLibrary.K2_UnPauseTimerHandle` (`self.TimerHandle`)))

(event `PauseEvent`
  (`KismetSystemLibrary.K2_PauseTimerHandle` (`self.TimerHandle`)))

(fn `UserConstructionScript`)