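; Strategy game mode for Starshot that runs the turn cycle between player, AI and environment.
; PlayerTurnCheck scans PlayerArray for remaining action points and calls CycleActivePlayer, which dispatches each turn event by index.
; AI and environment turns are placeholders that print and pass after a delay, with the environment turn refilling action points.
; The strategy controller, cached on BeginPlay, has click events disabled during the AI turn and re-enabled for the player's.
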(event `PlayerTurnCheck`
  (for _ (range 2) :!label _label
    (for _array_element (`self.PlayerArray`)
      (if (> (`/Game/Blueprints/GamePieces/Pawn_BaseType.CurrAP` _array_element) 0)
        (goto _label :!via `Break`)))
    (`self.CycleActivePlayer` 0)))

(event `self.ReceiveBeginPlay`
  (`KismetSystemLibrary.PrintString` "Switched to GameMode Strategy")
  (bind _aspc_starshot_controller_strategy (cast `/Game/Blueprints/GameSettings/PC_StarshotControllerStrategy` (`GameplayStatics.GetPlayerController` 0)))
  (set `self.PlayerController` _aspc_starshot_controller_strategy))

(event `CycleActivePlayer`
  (params (Source :type Integer))
  (switch `int` Source
    (:`0`
      (`self.AITurnEvent`))
    (:`1`
      (`self.EnvTurnEvent`))
    (:`2`
      (`self.PlayerTurnEvent` :!label _label_2))
    (:`4`
      (`KismetSystemLibrary.PrintString` "Cycle #4")
      (goto _label_2))))

(event `PlayerTurnEvent`
  (set `PlayerController.bEnableClickEvents` true (`self.PlayerController`)))

(event `AITurnEvent`
  (set `PlayerController.bEnableClickEvents` false (`self.PlayerController`))
  (`KismetSystemLibrary.PrintString` "Passing AI turn")
  (`KismetSystemLibrary.RetriggerableDelay` 1.0)
  (`self.CycleActivePlayer` 1))

(event `EnvTurnEvent`
  (`KismetSystemLibrary.PrintString` "Passing Env turn")
  (`KismetSystemLibrary.RetriggerableDelay` 1.0)
  (for _array_element (`self.PlayerArray`)
    (set `/Game/Blueprints/GamePieces/Pawn_BaseType.CurrAP` 2 _array_element))
  (`self.CycleActivePlayer` 2))

(fn `UserConstructionScript`)