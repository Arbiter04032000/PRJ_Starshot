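; GI_Starshot is the game instance for Starshot, holding the random event list, inventory and player fleet.
; On Init it collects event table rows flagged IsRandom into RandomEvents and prints them.
; AddShipToPlayerFleet copies a ship row's stored info and placeholder modules into PlayerFleet with an empty unique name.
; Inventory additions and the probe and print events write debug text to screen.
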(event `self.ReceiveInit`
  (`self.GetRandomEvents`)
  (for _array_element (`self.RandomEvents`)
    (`KismetSystemLibrary.PrintString` (`KismetStringLibrary.Conv_NameToString` _array_element))))

(event `GetRandomEvents`
  (bind _outrownames (`DataTableFunctionLibrary.GetDataTableRowNames` "/Game/Assets/Datatables/TextData/DTTD_Index.DTTD_Index"))
  (for _array_element _outrownames
    (bind _returnvalue (`|GetDataTableRow` "/Game/Assets/Datatables/TextData/DTTD_Index.DTTD_Index" _array_element)
      (:`then`
        (if (`.IsRandom?_33_82318CE649E5101BB659F1B80CB5403C` (break `/Game/Assets/Datatables/TextData/Struct_TextData` _returnvalue))
          (`KismetArrayLibrary.Array_Add` (`self.RandomEvents`) _array_element))))))

(event `InstanceProbeEvent`
  (`KismetSystemLibrary.PrintText` (`|FormatText` "Instance {0} present" (`KismetTextLibrary.Conv_StringToText` (`KismetSystemLibrary.GetObjectName` (`GameplayStatics.GetGameInstance`))))))

(event `PrintEvents`
  (for _array_element (`self.RandomEvents`)
    (`KismetSystemLibrary.PrintText` (`KismetTextLibrary.Conv_NameToText` _array_element))))

(event `AddToInventory`
  (params (StringToAdd :type Name))
  (bind _ldinventory (`self.LdInventory`))
  (bind _returnvalue (`KismetArrayLibrary.Array_Add` _ldinventory StringToAdd))
  (`KismetSystemLibrary.PrintText` (`|FormatText` "Added item {0} in slot {1}" (`KismetTextLibrary.Conv_StringToText` (`KismetStringLibrary.Conv_NameToString` (`|GetArrayItem` _ldinventory _returnvalue))) _returnvalue)))

(event `PrintInventory`
  (for _array_element (`self.LdInventory`)
    (`KismetSystemLibrary.PrintText` (`KismetTextLibrary.Conv_NameToText` _array_element))))

(fn `AddShipToPlayerFleet`
  (params (ShipToAdd :type Name))
  (bind _returnvalue (`|GetDataTableRow` "/Game/Blueprints/GamePieces/DTPSSI_Index.DTPSSI_Index" ShipToAdd)
    (:`then`
      (bind (_shipstoredinfo _uniquename _dummymodules) (break `/Game/Blueprints/GamePieces/Struct_PlayerShipStoredInfo` _returnvalue))
      (`KismetArrayLibrary.Array_Add` (`self.PlayerFleet`) (make `/Game/Blueprints/GamePieces/Struct_PlayerShipStoredInfo` _shipstoredinfo "" _dummymodules)))))