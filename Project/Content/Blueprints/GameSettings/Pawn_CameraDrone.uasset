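; Camera drone pawn that flies the player's view over the map and can spawn units for testing.
; Tick feeds the CameraX/CameraY axes, rotated by the root's yaw, into FloatingPawnMovement for horizontal movement.
; Holding middle mouse lets mouse movement turn controller yaw and pitch.
; NumPad 0 spawns a BP_Unit at the cursor hit, prints the hit actor's name and draws a persistent debug trace, whose result is unused.
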(event `self.ReceiveTick`
  (params (DeltaSeconds :type "Float (single-precision)"))
  (`PawnMovementComponent.AddInputVector` (`self.FloatingPawnMovement`) (`KismetMathLibrary.GreaterGreater_VectorRotator` (`KismetMathLibrary.MakeVector` (stale `InputAxis|CameraX` AxisValue) (stale `InputAxis|CameraY` AxisValue)) (`KismetMathLibrary.MakeRotator` 0.0 0.0 (.yaw (`SceneComponent.K2_GetComponentRotation` (`self.DefaultSceneRoot`))))) false))

(event `InputAxis|CameraX`
  (params (AxisValue :type "Float (single-precision)")))

(event `InputAxis|CameraY`
  (params (AxisValue :type "Float (single-precision)")))

(event `InputAxisKey|MouseX`
  (params (AxisValue :type "Float (single-precision)"))
  (if (stale `Key|MiddleMouseButton` _output_get)
    (`self.AddControllerYawInput` AxisValue)))

(event `Key|MiddleMouseButton`
  (params (Key :type "Key Structure"))
  (:`Pressed`
    (bind _output_get (set `self.CameraFreeRotate` true)))
  (:`Released`
    (set `self.CameraFreeRotate` false)))

(event `InputAxisKey|MouseY`
  (params (AxisValue :type "Float (single-precision)"))
  (if (stale `Key|MiddleMouseButton` _output_get)
    (`self.AddControllerPitchInput` AxisValue)))

(event `SpawnAtRet`
  (bind (_bblockinghit _binitialoverlap _time _distance _location _impactpoint _normal _impactnormal _physmat _hitactor) (`GameplayStatics.BreakHitResult` (`PlayerController.GetHitResultUnderCursorByChannel` (`GameplayStatics.GetPlayerController` 0) "TraceTypeQuery3" true)))
  (`KismetSystemLibrary.LineTraceSingle` :`Start` (`SceneComponent.K2_GetComponentLocation` (`self.Camera`)) :`TraceChannel` "TraceTypeQuery3" :`DrawDebugType` "Persistent")
  (`|SpawnActorFromClass` "/Game/AdvancedTurnBasedTileToolkit/Core/Units/BP_Unit.BP_Unit_C" (`KismetMathLibrary.MakeTransform` _location) "Undefined" "OverrideRootScale" null 2 2 6 1 0 100.0 100.0 35.0 0.0 false "NewEnumerator0" true null null)
  (`KismetSystemLibrary.PrintString` (`KismetSystemLibrary.GetObjectName` _hitactor)))

(event `Key|NumPadZero`
  (params (Key :type "Key Structure"))
  (:`Pressed`
    (`self.SpawnAtRet`)))

(fn `UserConstructionScript`)