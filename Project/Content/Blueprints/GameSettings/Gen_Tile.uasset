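; Gen_Tile is a tile actor that spawns, holds and tracks an occupying Pawn_BaseType.
; SpawnActor creates an actor of the given class and passes it to AttachActor, which ignores anything that is not a Pawn_BaseType.
; AttachActor clears the pawn's previous tile, attaches it with KeepRelative rules, and links tile and pawn through Occupant and OccupiedTile.
; Destroying the tile also destroys all its attached actors.
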(event `SpawnActor`
  (params (ActorClass :type "Actor Class Reference"))
  (bind _returnvalue (`|SpawnActorFromClass` ActorClass (`KismetMathLibrary.MakeTransform` (0.0 0.0 0.0)) "Undefined" "OverrideRootScale" null null))
  (`self.AttachActor` _returnvalue))

(event `self.ReceiveDestroyed`
  (for _array_element (`self.GetAttachedActors`)
    (`self.K2_DestroyActor` _array_element)))

(event `AttachActor`
  (params (ActorToAttach :type "Actor Object Reference"))
  (bind _aspawn_base_type (cast `/Game/Blueprints/GamePieces/Pawn_BaseType` ActorToAttach))
  (set `/Game/Blueprints/GameSettings/Gen_Tile.Occupant` null (`/Game/Blueprints/GamePieces/Pawn_BaseType.OccupiedTile` _aspawn_base_type))
  (`self.K2_AttachToActor` _aspawn_base_type self "None" "KeepRelative" "KeepRelative" "KeepRelative" true)
  (set `self.Occupant` _aspawn_base_type)
  (set `/Game/Blueprints/GamePieces/Pawn_BaseType.OccupiedTile` self _aspawn_base_type)
  (`KismetSystemLibrary.PrintString` "AttachedActor"))

(fn `UserConstructionScript`)