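; Player controller for Starshot's strategy mode that handles alternate-click commands for the selected pawn.
; It caches the strategy game mode on BeginPlay.
; Right mouse or X traces under the cursor and accepts a tile, or a pawn's occupied tile, only if it is among the selected pawn's ValidTiles.
; It then passes the hit actor, a pawn flag and the pawn class enum to that pawn's AltClickEvent.
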(event `self.ReceiveBeginPlay`
  (`parent.ReceiveBeginPlay`)
  (bind _asgm_starshot_strategy_bp (cast `/Game/Blueprints/GameSettings/GM_StarshotStrategyBP` (`GameplayStatics.GetGameMode`)))
  (set `self.Gamemode` _asgm_starshot_strategy_bp)
  (`KismetSystemLibrary.PrintText` (`|FormatText` "Switched to {playercontroller} at ID {ID}" (`KismetTextLibrary.Conv_ObjectToText` self) (`GameplayStatics.GetPlayerControllerID` null))))

(event `Key|X`
  (params (Key :type "Key Structure"))
  (bind (_bblockinghit _binitialoverlap _time _distance _location _impactpoint _normal _impactnormal _physmat _hitactor) (`GameplayStatics.BreakHitResult` (`self.GetHitResultUnderCursorByChannel` "TraceTypeQuery3")))
  (bind _selectedpawn (`/Game/Blueprints/GameSettings/GM_StarshotStrategyBP.SelectedPawn` (`self.Gamemode`)))
  (bind _validtiles (`/Game/Blueprints/GamePieces/Old/Pawn_BaseType.ValidTiles` _selectedpawn))
  (bind _returnvalue (`KismetMathLibrary.ClassIsChildOf` (`GameplayStatics.GetObjectClass` _hitactor) "/Game/Blueprints/GamePieces/Old/Pawn_BaseType.Pawn_BaseType_C"))
  (:`Pressed`
    (if (`KismetSystemLibrary.IsValid` _selectedpawn) :!label _label
      (bind _aspawn_base_type (cast `/Game/Blueprints/GamePieces/Old/Pawn_BaseType` _hitactor)
        (:`then`
          (`KismetSystemLibrary.PrintText` (`|FormatText` "{object} @ {vecLocation}" (`KismetTextLibrary.Conv_StringToText` (`KismetSystemLibrary.GetObjectName` _hitactor)) (`KismetTextLibrary.Conv_VectorToText` _impactpoint)))
          (if (> (`KismetArrayLibrary.Array_Find` _validtiles (`/Game/Blueprints/GamePieces/Old/Pawn_BaseType.OccupiedTile` _aspawn_base_type)) -1)
            (if (not _returnvalue) :!label _label_2
              (`/Game/Blueprints/GamePieces/Old/Pawn_BaseType.AltClickEvent` _selectedpawn _hitactor _returnvalue "NewEnumerator0")
              (else
                (bind _aspawn_base_type_2 (cast `/Game/Blueprints/GamePieces/Old/Pawn_BaseType` _hitactor)
                  (:`then`
                    (`/Game/Blueprints/GamePieces/Old/Pawn_BaseType.AltClickEvent` _selectedpawn _hitactor _returnvalue (`/Game/Blueprints/GamePieces/Old/Pawn_BaseType.Class` _aspawn_base_type_2)))
                  (:`CastFailed`
                    (`KismetSystemLibrary.PrintString` "Bad class" true true (struct :`R` 1.0 :`A` 1.0))))))))
        (:`CastFailed`
          (bind _asgen_tile (cast `/Game/Blueprints/GameSettings/Gen_Tile` _hitactor))
          (if (> (`KismetArrayLibrary.Array_Find` _validtiles _asgen_tile) -1)
            (goto _label_2)))))))

(event `Key|RightMouseButton` :consume false
  (params (Key :type "Key Structure"))
  (:`Pressed`
    (goto _label)))

(fn `UserConstructionScript`
  (`parent.UserConstructionScript`))