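; Grid generator actor that spawns an offset-column (hex-style) field of Gen_Tile actors, storing coordinates on each and attaching them to itself.
; SpawnTiles is bound to a grid dispatcher at BeginPlay and fills TilesArray, which FindTile indexes by flattened coordinate.
; Helper functions use column parity to resolve neighbours and directional steps, with events that highlight or print results.
; GetDistance is a stub, and random pawn spawning is disconnected.
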(event `self.ReceiveBeginPlay`
  (add `self.Grid_Dispatcher` (delegate `SpawnTiles`)))

(event `SpawnTiles`
  (bind (_x _y) (`KismetMathLibrary.BreakVector2D` (`self.GridSize`)))
  (for _index (range (+ (`KismetMathLibrary.FTrunc` _x) 1))
    (for _index_2 (range (+ (`KismetMathLibrary.FTrunc` _y) 1))
      (bind _returnvalue (* _index 112.5))
      (bind _returnvalue_2 (* _index_2 130.0))
      (bind _returnvalue_3 (`|SpawnActorFromClass` "/Game/Blueprints/GameSettings/Gen_Tile.Gen_Tile_C" (`KismetMathLibrary.MakeTransform` (`KismetMathLibrary.SelectVector` (`KismetMathLibrary.MakeVector` _returnvalue _returnvalue_2) (`KismetMathLibrary.MakeVector` _returnvalue (+ _returnvalue_2 65.0)) (== (mod _index 2) 0))) "Undefined" "OverrideRootScale" null null))
      (set `/Game/Blueprints/GameSettings/Gen_Tile.Coords` (`KismetMathLibrary.MakeVector2D` (`KismetMathLibrary.Conv_IntToDouble` _index) (`KismetMathLibrary.Conv_IntToDouble` _index_2)) _returnvalue_3)
      (`self.K2_AttachToActor` _returnvalue_3 self "None" "KeepWorld" "KeepWorld" "KeepWorld" false)
      (`KismetArrayLibrary.Array_Add` (`self.TilesArray`) _returnvalue_3))))

(event `ClearTiles`
  (bind _tilesarray (`self.TilesArray`))
  (for (_array_element _array_index) _tilesarray :!label _label
    (`self.K2_DestroyActor` _array_element)
    (`KismetArrayLibrary.Array_Remove` _tilesarray _array_index))
  (if (> (`KismetArrayLibrary.Array_Length` _tilesarray) 0)
    (goto _label)))

(event `GetTile`
  (params (TileToFind :type "Vector2D Structure"))
  (bind _outtile (`self.FindTile` TileToFind))
  (`KismetSystemLibrary.PrintText` (`|FormatText` "{0} {1}" (`KismetTextLibrary.Conv_StringToText` (`KismetSystemLibrary.GetObjectName` _outtile)) (`KismetTextLibrary.Conv_Vector2dToText` (`/Game/Blueprints/GameSettings/Gen_Tile.Coords` _outtile)))))

(event `GetDistance`
  (params (SourceCoords :type "Vector2D Structure" :default (0.0 3.0)) (TargetCoords :type "Vector2D Structure" :default (5.0 7.0)))
  (`KismetSystemLibrary.PrintString` "Hello"))

(event `GetNeighbourTilesEv`
  (params (Target :type "Vector2D Structure"))
  (bind (_outtiles _outtileobjs) (`self.GetNeighbourTiles` Target))
  (for _array_element _outtileobjs
    (`/Game/Blueprints/GameSettings/Gen_Tile.HighlightTile` _array_element 1)))

(event `GetCardinalDirEv`
  (params (`@` :type "Vector2D Structure" :default (2.0 0.0)) (To :type "Vector2D Structure" :default (5.0 0.0)))
  (bind _outdir (`self.GetCardinalDir` `@` To))
  (`KismetSystemLibrary.PrintText` (`KismetTextLibrary.Conv_Vector2dToText` _outdir)))

(event `GetTileInCardinalEv`
  (params (Target :type "Vector2D Structure") (Cardinal :type "Vector2D Structure"))
  (bind _coord (`self.GetTileInCardinal` Target Cardinal))
  (`KismetSystemLibrary.PrintText` (`|FormatText` "Neighbour of {0} @ {1} is {2}" (`KismetTextLibrary.Conv_Vector2dToText` Target) (`KismetTextLibrary.Conv_Vector2dToText` Cardinal) (`KismetTextLibrary.Conv_Vector2dToText` _coord)) true true (struct :`G` 0.66 :`B` 1.0 :`A` 1.0) 10.0))

(fn `FindTile`
  (params (InCoord :type "Vector2D Structure"))
  (returns (OutTile :type "/Game/Blueprints/GameSettings/Gen_Tile Object Reference"))
  (bind (_x _y) (`KismetMathLibrary.BreakVector2D` InCoord))
  (return (`|GetArrayItem` (`self.TilesArray`) (`KismetMathLibrary.FTrunc` (+ _y (* _x (+ (`.Y` (`KismetMathLibrary.BreakVector2D` (`self.GridSize`))) 1.0)))))))

(fn `GetCardinalDir`
  (params (Target :type "Vector2D Structure") (DirectTowards :type "Vector2D Structure"))
  (returns (OutDir :type "Vector2D Structure") (IsVertex :type Boolean))
  (bind (_x _y) (`KismetMathLibrary.BreakVector2D` Target))
  (bind (_x_2 _y_2) (`KismetMathLibrary.BreakVector2D` DirectTowards))
  (return (`KismetMathLibrary.MakeVector2D` (select `bool` (== _x _x_2) :`false` (select `bool` (< _x _x_2) :`false` -1.0 :`true` 1.0 :!type "Float (single-precision)")) (select `bool` (== _y _y_2) :`false` (select `bool` (< _y _y_2) :`false` -1.0 :`true` 1.0 :!type "Float (single-precision)"))) false))

(fn `GetNeighbourTiles`
  (params (Target :type "Vector2D Structure"))
  (returns (OutTiles :type "Array of Vector2D Structure") (OutTileObjs :type "Array of /Game/Blueprints/GameSettings/Gen_Tile Object Reference") (IsEdgeTile :type Boolean))
  (locals (bIsEdgeTile :type Boolean :default false) (ArrayToMake :type "Array of Vector2D Structure") (TileArrayToMake :type "Array of /Game/Blueprints/GameSettings/Gen_Tile Object Reference"))
  (bind (_x _y) (`KismetMathLibrary.BreakVector2D` Target))
  (bind _arraytomake (`local.ArrayToMake`))
  (bind _returnvalue (- _x 1.0))
  (bind (_x_2 _y_2) (`KismetMathLibrary.BreakVector2D` (`self.GridSize`)))
  (bind _returnvalue_2 (+ _x 1.0))
  (bind _returnvalue_3 (select `bool` (> (mod (`KismetMathLibrary.FTrunc` _x) 2) 0) :`false` -1.0 :`true` 1.0 :!type "Float (single-precision)"))
  (bind _output_get (set `local.ArrayToMake` (`|MakeArray` (`KismetMathLibrary.MakeVector2D` _x (+ _y 1.0)) (`KismetMathLibrary.MakeVector2D` _x (- _y 1.0)) (`KismetMathLibrary.MakeVector2D` _returnvalue_2 _y) (`KismetMathLibrary.MakeVector2D` _returnvalue_2 (+ _y _returnvalue_3)) (`KismetMathLibrary.MakeVector2D` _returnvalue _y) (`KismetMathLibrary.MakeVector2D` _returnvalue (+ _y _returnvalue_3)))))
  (for _array_element _output_get
    (`KismetSystemLibrary.PrintText` (`|FormatText` "Sanity Checking {0}" (`KismetTextLibrary.Conv_Vector2dToText` _array_element)))
    (bind (_x_3 _y_3) (`KismetMathLibrary.BreakVector2D` _array_element))
    (if (or (> _x_3 _x_2) (<= _x_3 -1.0) (> _y_3 _y_2) (<= _y_3 -1.0))
      (bind _returnvalue_4 (`KismetArrayLibrary.Array_RemoveItem` (`local.ArrayToMake`) _array_element))
      (set `local.bIsEdgeTile` _returnvalue_4)))
  (for _array_element_2 _arraytomake
    (bind _outtile (`self.FindTile` _array_element_2))
    (if (`KismetSystemLibrary.IsValid` _outtile)
      (`KismetArrayLibrary.Array_Add` (`local.TileArrayToMake`) _outtile)))
  (return _arraytomake (`local.TileArrayToMake`) (`local.bIsEdgeTile`)))

(fn `GetTileInCardinal`
  (params (Target :type "Vector2D Structure") (Cardinal :type "Vector2D Structure"))
  (returns (Coord :type "Vector2D Structure") (Tile :type "/Game/Blueprints/GameSettings/Gen_Tile Object Reference"))
  (bind (_x _y) (`KismetMathLibrary.BreakVector2D` Target))
  (bind (_x_2 _y_2) (`KismetMathLibrary.BreakVector2D` Cardinal))
  (bind _returnvalue (> (mod (`KismetMathLibrary.FTrunc` _x) 2) 0))
  (bind _returnvalue_2 (not _returnvalue))
  (return (`KismetMathLibrary.MakeVector2D` (+ _x _x_2) (+ _y (select `bool` (== _x_2 0.0) :`false` (select `bool` _returnvalue_2 :`false` (select `bool` (and _returnvalue (< _y_2 0.0)) :`true` -1.0 :!type "Float (single-precision)") :`true` (select `bool` (and _returnvalue_2 (> _y_2 0.0)) :`true` 1.0 :!type "Float (single-precision)")) :`true` (select `bool` (== _y_2 0.0) :`false` (select `bool` (>= _y_2 0.0) :`false` -1.0 :`true` 1.0 :!type "Float (single-precision)"))))) null))

(fn `UserConstructionScript`)